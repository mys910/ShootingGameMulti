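; Player state for the shooting game that holds each player's HP and Armor, with functions to damage, heal and add armor.
; Armor absorbs a hit it can survive; otherwise it drops to zero and HP takes the full damage.
; RepNotify functions print the new values and fire event dispatchers with current and max values.
; An older path that updated the name tag and HUD directly is left disconnected.
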(event EventBeginPlay)

(event EventTick
  (params (DeltaSeconds :type Float%20%28single-precision%29)))

(fn ConstructionScript)

(fn AddDamage
  (params (Damage :type Float%20%28single-precision%29))
  (if (> (- (Variables|Default|GetArmor) Damage) 0.0)
    (Variables|Default|SetArmor (Math|Float|Clamp(Float) (- (Variables|Default|GetArmor) Damage) 0.0 1e+02))
    (else
      (Variables|Default|SetArmor 0.0)
      (Variables|Default|SetHP (Math|Float|Clamp(Float) (- (Variables|Default|GetHP) Damage) 0.0 1e+02)))))

(fn OnRepHP
  ;[1 1 1] Client
  (Development|PrintString (Utilities|String|Append "OnRepHp-" (Utilities|String|ToString(Float) (Variables|Default|GetHP))))
  (Default|CallNewEventDispatcherHP (Variables|Default|GetHP) 1e+02))

(fn AddHeal
  (params (Heal :type Float%20%28single-precision%29))
  (Variables|Default|SetHP (Math|Float|Clamp(Float) (+ (Variables|Default|GetHP) Heal) 0.0 1e+02)))

(fn OnRepArmor
  (Development|PrintString (Utilities|String|Append "OnRepArmor-" (Utilities|String|ToString(Float) (Variables|Default|GetArmor))))
  (Default|CallNewEventDispatcherArmor (Variables|Default|GetArmor) 1e+02))

(fn AddArmor
  (params (Armor :type Float%20%28single-precision%29))
  (Variables|Default|SetArmor (Math|Float|Clamp(Float) (+ Armor (Variables|Default|GetArmor)) 0.0 1e+02)))