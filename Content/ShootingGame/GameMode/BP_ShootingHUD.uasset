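; BP_ShootingHUD is the shooting game's HUD, which creates the ShootingWidget on BeginPlay and sets game-only input with the cursor hidden.
; It binds to BP_ShootingPlayerState's HP and Armor dispatchers, retrying on a 0.1-second timer until the player state cast succeeds.
; Update functions forward ammo, magazine, HP, armor, and the position and visibility of an F guide prompt to the widget.
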(event EventBeginPlay
  (bind _returnvalue (Game|GetPlayerController 0))
  (bind _returnvalue_2 (UserInterface|CreateWidget "/Game/ShootingGame/Widget/ShootingWidget.ShootingWidget_C"))
  (bind _output_get (Variables|Default|SetHUD_Widget _returnvalue_2))
  (UserInterface|Viewport|AddtoViewport _output_get 0)
  (CallFunction|BindPlayerState)
  (Input|SetInputModeGameOnly _returnvalue)
  (Variables|/Script/Engine.PlayerController|SetbShowMouseCursor _returnvalue false))

(fn ConstructionScript)

(fn UpdateAMMO
  (params (NewParam :type Integer))
  (Default|SetAMMO (Variables|Default|GetHUD_Widget) NewParam))

(fn UpdateMAG
  (params (MAG :type Integer))
  (Default|SetMAG (Variables|Default|GetHUD_Widget) MAG))

(fn UpdateHP
  (params (Cur_HP :type Float%20%28single-precision%29) (MAX_HP :type Float%20%28single-precision%29))
  (Default|SetHP (Variables|Default|GetHUD_Widget) Cur_HP MAX_HP))

(fn UpdateGuideF
  (params (WorldLocatioon :type Vector))
  (Default|SetPositionGuideF (Variables|Default|GetHUD_Widget) WorldLocatioon))

(fn SetVisibilityGuideF
  (params (InVisibility :type ESlateVisibility%20Enum :default "Visible"))
  (Default|SetVisibilityGuideF (Variables|Default|GetHUD_Widget) InVisibility))

(fn BindPlayerState
  (bind _asbp_shooting_player_state (Utilities|Casting|CastToBP_ShootingPlayerState (Variables|/Script/Engine.Controller|GetPlayerState (Game|GetPlayerController 0)))
    (:then
      (EventDispatchers|BindEventtoNewEventDispatcherHP _asbp_shooting_player_state (EventDispatchers|CreateEvent :!event UpdateHP))
      (EventDispatchers|BindEventtoNewEventDispatcherArmor _asbp_shooting_player_state (EventDispatchers|CreateEvent :!event UpdateArmor)))
    (:CastFailed
      (Utilities|Time|SetTimerbyFunctionName 0 "BindPlayerState" 0.1))))

(fn UpdateArmor
  (params (CurArmor :type Float%20%28single-precision%29) (MaxArmor :type Float%20%28single-precision%29))
  (Default|SetArmor (Variables|Default|GetHUD_Widget) CurArmor MaxArmor))