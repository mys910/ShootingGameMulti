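; BP_HealArea is a healing zone actor that periodically restores health to shooting-game characters standing inside it.
; A looping one-second timer started on BeginPlay calls HealOverlapPlayer, which gathers BP_ShootingCharacter actors overlapping its Sphere.
; Each living character receives a fixed heal through AddHeal on its BP_ShootingPlayerState.
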(event EventBeginPlay
  (Utilities|Time|SetTimerbyFunctionName 0 "HealOverlapPlayer" 1.0 true))

(fn ConstructionScript)

(fn HealOverlapPlayer
  (for _array_element (Collision|GetOverlappingActors (Variables|Default|GetSphere) "/Game/ShootingGame/GameMode/BP_ShootingCharacter.BP_ShootingCharacter_C" :!class /Script/Engine.PrimitiveComponent)
    (bind _asbp_shooting_character (Utilities|Casting|CastToBP_ShootingCharacter _array_element))
    (if (not (Default|IsDie _asbp_shooting_character))
      (bind _asbp_shooting_player_state (Utilities|Casting|CastToBP_ShootingPlayerState (Variables|/Script/Engine.Pawn|GetPlayerState _asbp_shooting_character)))
      (Default|AddHeal _asbp_shooting_player_state 1e+01))))