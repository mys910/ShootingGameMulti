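; Networked pickup rifle that attaches to a shooting character's weapon socket, swapping out any held weapon, with mesh, damage and ammo capacity from WeaponRef.
; A looping timer replays the shoot montage; fire notifies spawn muzzle effects and make the local player request a server camera-forward line trace that damages actors and destructibles.
; Remote clients predict ammo use, OnRep updates the HUD, and reload notifies consume a magazine server-side to refill ammo.
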(event Custom|Req_HitCheck
  (params (Location :type Vector) (Forward :type Vector))
  (CallFunction|ServerHitCheck Location Forward))

(event Custom|ReqReload
  (CallFunction|ServerUseMag))

(event EventBeginPlay
  (bind _weaponref (Variables|Default|GetWeaponRef))
  (Components|StaticMesh|SetStaticMesh (Variables|Default|GetStaticMesh) (.staticmesh _weaponref))
  (Variables|Default|SetAMMO (.maxammo _weaponref)))

(fn ConstructionScript)

(fn AttachtoCharacter
  (params (Character :type Character%20Object%20Reference))
  (bind _staticmesh (Variables|Default|GetStaticMesh))
  (Physics|SetSimulatePhysics _staticmesh false)
  (Collision|SetCollisionEnabled _staticmesh "QueryAndPhysics")
  (Transformation|AttachComponentToComponent (Variables|/Script/Engine.Character|GetMesh Character) "weapon" "SnapToTarget" "SnapToTarget" "KeepWorld" true)
  (bind _asbp_shooting_character (Utilities|Casting|CastToBP_ShootingCharacter Character))
  (bind _output_get (Variables|Default|SetOwnCharacter _asbp_shooting_character))
  (Variables|/Game/ShootingGame/GameMode/BP_ShootingCharacter.BP_ShootingCharacter_C|SetAttachedWeapon _output_get self)
  (Variables|/Script/Engine.Pawn|SetbUseControllerRotationYaw _asbp_shooting_character true)
  (Variables|/Script/Engine.CharacterMovementComponent|SetbOrientRotationToMovement (Variables|/Script/Engine.Character|GetCharacterMovement _asbp_shooting_character) false)
  (CallFunction|UpdateAmmo (Variables|Default|GetAMMO)))

(fn DetachtoCharacter
  (params (Character :type Character%20Object%20Reference))
  (bind _staticmesh (Variables|Default|GetStaticMesh))
  (Transformation|DetachFromActor "KeepWorld" "KeepWorld" "KeepWorld")
  (Collision|SetCollisionEnabled _staticmesh "QueryAndPhysics")
  (Physics|SetSimulatePhysics _staticmesh true)
  (CallFunction|UpdateAmmo)
  ;[1 1 1] UnEquip 상태로 정보 변경
  (bind _asbp_shooting_character (Utilities|Casting|CastToBP_ShootingCharacter Character))
  (Variables|/Game/ShootingGame/GameMode/BP_ShootingCharacter.BP_ShootingCharacter_C|SetAttachedWeapon _asbp_shooting_character 0)
  (Variables|Default|SetOwnCharacter 0)
  (Variables|/Script/Engine.Pawn|SetbUseControllerRotationYaw _asbp_shooting_character false)
  (Variables|/Script/Engine.CharacterMovementComponent|SetbOrientRotationToMovement (Variables|/Script/Engine.Character|GetCharacterMovement _asbp_shooting_character) true))

(fn PullTriger
  (params (Character :type Character%20Object%20Reference))
  (if (not (<= (Variables|Default|GetAMMO) 0))
    (Animation|PlayAnimMontage Character "/Game/RifleAnimsetPro/Animations/InPlace/Rifle_ShootOnce_Montage.Rifle_ShootOnce_Montage" 1.0 "None")
    (Utilities|Time|SetTimerbyFunctionName 0 "AddShoot" 0.1 true)))

(fn AddShoot
  (bind _owncharacter (Variables|Default|GetOwnCharacter))
  (Utilities|IsValid _owncharacter
    (:Is%20Valid
      (Animation|PlayAnimMontage _owncharacter "/Game/RifleAnimsetPro/Animations/InPlace/Rifle_ShootOnce_Montage.Rifle_ShootOnce_Montage" 1.0 "None"))
    (:Is%20Not%20Valid
      (Utilities|Time|ClearTimerbyFunctionName 0 "AddShoot"))))

(fn ReleaseTriger
  (Utilities|Time|ClearTimerbyFunctionName 0 "AddShoot"))

(fn EventNotifyFire
  (bind _returnvalue (Game|GetPlayerCameraManager 0))
  (bind _staticmesh (Variables|Default|GetStaticMesh))
  ;[1 1 1] Client
  (if (not (<= (Variables|Default|GetAMMO) 0))
    (Effects|SpawnEmitteratLocation "/Game/StarterContent/Particles/P_Explosion.P_Explosion" (Transformation|GetSocketLocation _staticmesh "Muzzle") (Transformation|GetSocketRotation _staticmesh "Muzzle"))
    (Audio|Components|Audio|Play (Variables|Default|GetAudio) 0.0)
    (Utilities|CheckMyPlayer
      (:True
        (Networking|SwitchHasAuthority
          (:Authority
            (if (CallFunction|CanUseAmmo)
              (CallFunction|ReqHitCheck (Transformation|GetActorLocation _returnvalue) (Transformation|GetActorForwardVector _returnvalue) :!label _label)))
          (:Remote
            (bind _is_used_ammo (CallFunction|UseAmmo))
            (if _is_used_ammo
              (goto _label))))))))

(fn UseAmmo
  (if (CallFunction|CanUseAmmo)
    (bind _result (Math|Integer|DecrementInt (Variables|Default|GetAMMO))
      (:%20%20
        (CallFunction|UpdateAmmo _result)
        (return true)))
    (else
      (return false))))

(fn UpdateAmmo
  (params (Value :type Integer))
  (Utilities|IsValid (Variables|Default|GetOwnCharacter)
    (:Is%20Valid
      (Utilities|CheckMyPlayer
        (:True
          (bind _asbp_shooting_hud (Utilities|Casting|CastToBP_ShootingHUD (HUD|GetHUD (Game|GetPlayerController 0))))
          (Default|UpdateAMMO _asbp_shooting_hud Value))))))

(fn DoReload
  (bind _owncharacter (Variables|Default|GetOwnCharacter))
  (Utilities|IsValid _owncharacter
    (:Is%20Valid
      (if (Default|HasMAG _owncharacter)
        (Animation|PlayAnimMontage _owncharacter "/Game/RifleAnimsetPro/Animations/InPlace/Rifle_Reload_2_Montage.Rifle_Reload_2_Montage" 1.0 "None")))))

(fn EventNotifyReload
  (Utilities|CheckMyPlayer
    (:True
      (CallFunction|ReqReload))))

(fn StopShot
  (Utilities|Time|SetTimerbyFunctionName 0 "AddShoot" 0.0))

(fn DoShoot
  (params (Character :type Character%20Object%20Reference))
  (if (not (<= (Variables|Default|GetAMMO) 0))
    (Animation|PlayAnimMontage Character "/Game/RifleAnimsetPro/Animations/InPlace/Rifle_ShootOnce_Montage.Rifle_ShootOnce_Montage" 1.0 "None")
    (Utilities|Time|SetTimerbyFunctionName 0 "AddShoot" 0.1 true)))

(fn CanUseAmmo
  (return (> (Variables|Default|GetAMMO) 0)))

(fn ServerHitCheck
  (params (Location :type Vector) (Forward :type Vector))
  (bind _is_used_ammo (CallFunction|UseAmmo))
  (if _is_used_ammo
    (bind _outhit (Collision|LineTraceForObjects (+ Location (* Forward 3.8e+02)) (+ Location (* Forward 2e+03)) (Utilities|Array|MakeArray "ObjectTypeQuery1" "ObjectTypeQuery2" "ObjectTypeQuery3" "ObjectTypeQuery4" "ObjectTypeQuery5" "ObjectTypeQuery6") false 0 "Persistent"))
    (Utilities|FlowControl|Sequence
      (:then_0
        (Game|Damage|ApplyDamage (.HitActor (Collision|BreakHitResult _outhit)) (.damage (Variables|Default|GetWeaponRef)) (Pawn|GetController (Variables|Default|GetOwnCharacter)) self))
      (:then_1
        (bind _asdestructible_component (Utilities|Casting|CastToDestructibleComponent (.HitComponent (Collision|BreakHitResult _outhit))))
        (Class|DestructibleComponent|ApplyDamage _asdestructible_component 5e+01 (.Location (Collision|BreakHitResult _outhit)) (.ImpactPoint (Collision|BreakHitResult _outhit)) 2e+04)))))

(fn OnRepAMMO
  (CallFunction|UpdateAmmo (Variables|Default|GetAMMO)))

(fn ServerUseMag
  (bind _is_used_mag (Default|UseMAG (Variables|Default|GetOwnCharacter)))
  (if _is_used_mag
    (CallFunction|SetAmmo (.maxammo (Variables|Default|GetWeaponRef)))))

(fn SetAmmo
  (params (Ammo :type Integer))
  (bind _output_get (Variables|Default|SetAMMO Ammo))
  (CallFunction|UpdateAmmo _output_get))

(fn EventCanPickUp
  (return (not (Utilities|IsValid (Variables|Default|GetOwnCharacter)))))

(fn EventPress
  (params (Character :type Character%20Object%20Reference))
  (bind _asbp_shooting_character (Utilities|Casting|CastToBP_ShootingCharacter Character))
  (Utilities|IsValid (Variables|/Game/ShootingGame/GameMode/BP_ShootingCharacter.BP_ShootingCharacter_C|GetAttachedWeapon _asbp_shooting_character)
    (:Is%20Valid
      (CallFunction|DetachtoCharacter (Variables|/Game/ShootingGame/GameMode/BP_ShootingCharacter.BP_ShootingCharacter_C|GetAttachedWeapon _asbp_shooting_character) Character))
    (:Is%20Not%20Valid
      _))
  (CallFunction|AttachtoCharacter Character)
  (return true))

(fn EventRelease
  (params (Character :type Character%20Object%20Reference))
  (return false))