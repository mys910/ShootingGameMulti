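; BP_RotateBox is an actor whose cube can be set spinning and stopped by a character's press event.
; EventPress calls EnablePlay to toggle IsPlay and returns false, while EventRelease only returns false.
; While IsPlay is set, Tick adds relative yaw to the cube, scaled from DeltaSeconds plus TimeSec, so the step is not purely delta-time based.
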(event EventBeginPlay)

(event Collision|EventActorBeginOverlap
  (params (OtherActor :type Actor%20Object%20Reference)))

(event EventTick
  (params (DeltaSeconds :type Float%20%28single-precision%29))
  (if (Variables|Default|GetIsPlay)
    (Transformation|AddRelativeRotation (Variables|Default|GetCube) (Math|Rotator|MakeRotator 0.0 0.0 (* (+ DeltaSeconds (Variables|Default|GetTimeSec)) 1e+02)) false false)))

(fn ConstructionScript)

(fn EnablePlay
  (Variables|Default|SetIsPlay (not (Variables|Default|GetIsPlay))))

(fn EventPress
  (params (Character :type Character%20Object%20Reference))
  (CallFunction|EnablePlay)
  (return false))

(fn EventRelease
  (params (Character :type Character%20Object%20Reference))
  (return false))