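; Burst-fire weapon Blueprint that plays three single-shot rifle montages per trigger pull.
; PullTriger checks AMMO, plays the first montage on the passed Character, then starts a looping AddShoot timer.
; AddShoot replays the montage on OwnCharacter while its counter lasts, then clears the timer.
; ReleaseTriger is empty, so releasing does not interrupt a burst, and ammo is not rechecked or decremented here.
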(fn ConstructionScript
  (|CallParentFunction))

(fn PullTriger
  (params (Character :type Character%20Object%20Reference))
  (if (not (<= (Variables|Default|GetAMMO) 0))
    (Animation|PlayAnimMontage Character "/Game/RifleAnimsetPro/Animations/InPlace/Rifle_ShootOnce_Montage.Rifle_ShootOnce_Montage" 1.0 "None")
    (Variables|Default|SetAddShootCount 2)
    (Utilities|Time|SetTimerbyFunctionName 0 "AddShoot" 0.2 true)))

(fn AddShoot
  (bind _owncharacter (Variables|Default|GetOwnCharacter))
  (Utilities|IsValid _owncharacter
    (:Is%20Valid
      (if (< 0 (Variables|Default|GetAddShootCount))
        (Animation|PlayAnimMontage _owncharacter "/Game/RifleAnimsetPro/Animations/InPlace/Rifle_ShootOnce_Montage.Rifle_ShootOnce_Montage" 1.0 "None")
        (Math|Integer|DecrementInt (Variables|Default|GetAddShootCount))
        (else
          (Utilities|Time|ClearTimerbyFunctionName 0 "AddShoot"))))))

(fn ReleaseTriger)